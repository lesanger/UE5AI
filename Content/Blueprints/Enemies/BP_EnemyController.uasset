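; AI controller for enemies that runs the BT_Enemy behavior tree and feeds its blackboard from AI perception.
; Each perception update passes to separate sight and hearing handlers, which filter by sense class.
; Sight tracks only player 0, setting TargetActor while seen, then clearing it and storing LastKnownLocation when sight is lost.
; Hearing writes the location of any heard stimulus to TargetLocation, regardless of its source.
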(event `self.ReceiveBeginPlay`
  (`self.RunBehaviorTree` "/Game/Blueprints/Enemies/BT_Enemy.BT_Enemy"))

(event `self.AIPerception.OnTargetPerceptionUpdated`
  (params (Actor :type "Actor Object Reference") (Stimulus :type "AIStimulus Structure"))
  (`self.HandleSightSense` Actor Stimulus)
  (`self.HandleHearingSense` Actor Stimulus))

(fn `HandleHearingSense`
  (params (InActor :type "Actor Object Reference") (InStimulus :type "AIStimulus Structure"))
  (bind (_instimulus_age _instimulus_expirationage _instimulus_strength _instimulus_stimuluslocation) (break `AIStimulus` (`local.InStimulus`)))
  (bind _returnvalue (`AIPerceptionSystem.GetSenseClassForStimulus` InStimulus))
  (if (== _returnvalue "/Script/AIModule.AISense_Hearing")
    (`BlackboardComponent.SetValueAsVector` (`self.Blackboard`) "TargetLocation" _instimulus_stimuluslocation)
    (else
      (return))))

(fn `HandleSightSense`
  (params (InActor :type "Actor Object Reference") (InStimulus :type "AIStimulus Structure"))
  (bind (_instimulus_age _instimulus_expirationage _instimulus_strength _instimulus_stimuluslocation) (break `AIStimulus` (`local.InStimulus`)))
  (bind (_instimulus_age_2 _instimulus_expirationage_2 _instimulus_strength_2 _instimulus_stimuluslocation_2 _instimulus_receiverlocation _instimulus_tag _instimulus_bsuccessfullysensed) (break `AIStimulus` (`local.InStimulus`)))
  (bind (_instimulus_age_3 _instimulus_expirationage_3 _instimulus_strength_3 _instimulus_stimuluslocation_3 _instimulus_receiverlocation_2 _instimulus_tag_2 _instimulus_bsuccessfullysensed_2) (break `AIStimulus` (`local.InStimulus`)))
  (bind _returnvalue (`AIPerceptionSystem.GetSenseClassForStimulus` InStimulus))
  (if (== _returnvalue "/Script/AIModule.AISense_Sight")
    (if (== (`local.InActor`) (`GameplayStatics.GetPlayerCharacter` 0))
      (`BlackboardComponent.SetValueAsObject` (`self.Blackboard`) "TargetActor" (`KismetMathLibrary.SelectObject` (`local.InActor`) null _instimulus_bsuccessfullysensed))
      (if (not _instimulus_bsuccessfullysensed_2)
        (`BlackboardComponent.SetValueAsVector` (`self.Blackboard`) "LastKnownLocation" _instimulus_stimuluslocation))
      (else
        (return)))
    (else
      (return))))

(fn `UserConstructionScript`)